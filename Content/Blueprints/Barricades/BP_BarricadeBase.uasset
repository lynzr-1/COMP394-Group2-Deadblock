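; Base barricade actor that starts at full health and takes damage from zombies.
; When its collider begins overlapping a BP_ZombieMaster, it confirms contact with that zombie's PlayerDetectCollider and subtracts ZombieDamage once per overlap.
; Only health exactly equal to zero triggers destruction, so overshooting below zero leaves it intact.
; Destruction moves it to a hard-coded world location and rotation, disables collider collision, and removes the actor after a short timer.
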(event OnComponentBeginOverlap(BarricadeCollider)
  (params (OverlappedComponent :type Primitive%20Component%20Object%20Reference) (OtherActor :type Actor%20Object%20Reference) (OtherComp :type Primitive%20Component%20Object%20Reference) (OtherBodyIndex :type Integer) (bFromSweep :type Boolean) (SweepResult :type Hit%20Result%20Structure%20%28by%20ref%29))
  (bind _asbp_zombie_master (Utilities|Casting|CastToBP_ZombieMaster OtherActor))
  (if (Class|PrimitiveComponent|IsOverlappingComponent (Variables|Default|GetBarricadeCollider) (Variables|/Game/Imports/Zombies/BP_ZombieMaster.BP_ZombieMaster_C|GetPlayerDetectCollider _asbp_zombie_master))
    (if (Variables|Default|GetisIntact)
      (CallFunction|TakeDamage (Variables|/Game/Imports/Zombies/BP_ZombieMaster.BP_ZombieMaster_C|GetZombieDamage _asbp_zombie_master)))))

(event EventBeginPlay
  (Variables|Default|SetBarricadeCurrentHealth (Variables|Default|GetBarricadeMaxHealth))
  (Variables|Default|SetisIntact true))

(event Collision|EventActorBeginOverlap
  (params (OtherActor :type Actor%20Object%20Reference)))

(event EventTick
  (params (DeltaSeconds :type Float%20%28single-precision%29)))

(fn ConstructionScript)

(fn TakeDamage
  (params (IncomingDamage :type Float%20%28double-precision%29%20%28by%20ref%29))
  (if (Variables|Default|GetisIntact)
    (bind _output_get (Variables|Default|SetBarricadeCurrentHealth (- (Variables|Default|GetBarricadeCurrentHealth) IncomingDamage)))
    (if (== _output_get 0.0)
      (Variables|Default|SetisIntact false)
      (CallFunction|Destroyed))))

(fn Destroyed
  (Transformation|SetActorLocationAndRotation "-90.0,0.0,0.0" "0.000000,0.000000,-90.000000")
  (Collision|SetCollisionEnabled (Variables|Default|GetBarricadeCollider) "NoCollision")
  (Utilities|Time|SetTimerbyFunctionName 0 "RemoveBarrierFromScene" 5.0))

(fn RemoveBarrierfromScene
  (Actor|DestroyActor))