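; Base zombie Blueprint that tracks health and takes damage from bullets.
; Health starts at its maximum on BeginPlay, and a BP_Bullet overlapping IncomingDamageCollider triggers TakeDamage.
; TakeDamage subtracts the damage of player 0's current weapon rather than reading it from the bullet.
; Health values print to screen for debugging, and no death handling exists here.
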(event OnComponentBeginOverlap(IncomingDamageCollider)
  (params (OverlappedComponent :type Primitive%20Component%20Object%20Reference) (OtherActor :type Actor%20Object%20Reference) (OtherComp :type Primitive%20Component%20Object%20Reference) (OtherBodyIndex :type Integer) (bFromSweep :type Boolean) (SweepResult :type Hit%20Result%20Structure%20%28by%20ref%29))
  (Utilities|Casting|CastToBP_Bullet OtherActor)
  (CallFunction|TakeDamage))

(event EventBeginPlay
  (bind _output_get (Variables|Default|SetZombieCurrentHealth (Variables|Default|GetZombieMaxHealth)))
  (Development|PrintString (Utilities|String|Append "Initial Zombie Health: " (Utilities|String|ToString(Float) _output_get))))

(event Collision|EventActorBeginOverlap
  (params (OtherActor :type Actor%20Object%20Reference)))

(event EventTick
  (params (DeltaSeconds :type Float%20%28single-precision%29)))

(fn ConstructionScript)

(fn TakeDamage
  (bind _asbp_player_character (Utilities|Casting|CastToBP_PlayerCharacter (Game|GetPlayerCharacter 0)))
  (bind _weapondamage (Default|GetWeaponDamage (Variables|/Game/Imports/PlayerCharacter/BP_PlayerCharacter.BP_PlayerCharacter_C|GetCurrentWeapon _asbp_player_character)))
  (bind _output_get (Variables|Default|SetZombieCurrentHealth (- (Variables|Default|GetZombieCurrentHealth) _weapondamage)))
  (Development|PrintString (Utilities|String|Append "Zombie Current Health: " (Utilities|String|ToString(Float) _output_get))))