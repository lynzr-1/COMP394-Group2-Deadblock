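; BP_ConsumableBase is a consumable pickup that restores the player character's health or stamina when interacted with.
; The Interact event switches on ConsumableType to call Heal or RestoreStamina.
; Each casts player 0 to BP_PlayerCharacter, adds its amount to the current stat clamped to the maximum, prints a debug message and destroys the actor.
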(event EventInteract
  (switch Utilities|FlowControl|Switch|SwitchonE_ConsumableType (Variables|Default|GetConsumableType)
    (:NewEnumerator0
      (CallFunction|Heal)
      (Development|PrintString "Healing Item Used"))
    (:NewEnumerator1
      (CallFunction|RestoreStamina))))

(fn ConstructionScript)

(fn Heal
  (bind _healingamount (Variables|Default|GetHealingAmount))
  (bind _asbp_player_character (Utilities|Casting|CastToBP_PlayerCharacter (Game|GetPlayerCharacter 0)))
  (bind _output_get (Variables|/Game/Imports/PlayerCharacter/BP_PlayerCharacter.BP_PlayerCharacter_C|SetCurrentHealth _asbp_player_character (Math|Float|Clamp(Float) (+ (Variables|/Game/Imports/PlayerCharacter/BP_PlayerCharacter.BP_PlayerCharacter_C|GetCurrentHealth _asbp_player_character) _healingamount) 0.0 (Variables|/Game/Imports/PlayerCharacter/BP_PlayerCharacter.BP_PlayerCharacter_C|GetMaxHealth _asbp_player_character))))
  (Development|PrintString (Utilities|String|Append "Healed for: " (Utilities|String|ToString(Float) _healingamount) " | Current Health: " (Utilities|String|ToString(Float) _output_get)))
  (Actor|DestroyActor))

(fn RestoreStamina
  (bind _staminaamount (Variables|Default|GetStaminaAmount))
  (bind _asbp_player_character (Utilities|Casting|CastToBP_PlayerCharacter (Game|GetPlayerCharacter 0)))
  (bind _output_get (Variables|/Game/Imports/PlayerCharacter/BP_PlayerCharacter.BP_PlayerCharacter_C|SetCurrentStamina _asbp_player_character (Math|Float|Clamp(Float) (+ (Variables|/Game/Imports/PlayerCharacter/BP_PlayerCharacter.BP_PlayerCharacter_C|GetCurrentStamina _asbp_player_character) _staminaamount) 0.0 (Variables|/Game/Imports/PlayerCharacter/BP_PlayerCharacter.BP_PlayerCharacter_C|GetMaxStamina _asbp_player_character))))
  (Development|PrintString (Utilities|String|Append "Restored: " (Utilities|String|ToString(Float) _staminaamount) "points of Stamina | Current Stamina: " (Utilities|String|ToString(Float) _output_get)))
  (Actor|DestroyActor))