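; Bullet actor that damages BP_ZombieMaster actors on overlap and destroys itself after a short delay.
; GetSourceWeaponDamage reads WeaponDamage from player 0's CurrentWeapon.
; The construction script stores that value in BulletDamage, but the overlap queries it again, so damage follows the weapon held at impact.
; Overlaps with other actors neither apply damage nor destroy the bullet.
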(event OnComponentBeginOverlap(BulletCollider)
  (params (OverlappedComponent :type Primitive%20Component%20Object%20Reference) (OtherActor :type Actor%20Object%20Reference) (OtherComp :type Primitive%20Component%20Object%20Reference) (OtherBodyIndex :type Integer) (bFromSweep :type Boolean) (SweepResult :type Hit%20Result%20Structure%20%28by%20ref%29))
  (bind _asbp_zombie_master (Utilities|Casting|CastToBP_ZombieMaster OtherActor))
  (bind _sourceweapondamage (CallFunction|GetSourceWeaponDamage))
  (Default|TakeDamage _asbp_zombie_master _sourceweapondamage)
  (Utilities|FlowControl|Delay 0.1)
  (Actor|DestroyActor))

(event EventTick
  (params (DeltaSeconds :type Float%20%28single-precision%29)))

(fn ConstructionScript
  (bind _sourceweapondamage (CallFunction|GetSourceWeaponDamage))
  (Variables|Default|SetBulletDamage _sourceweapondamage))

(fn GetSourceWeaponDamage
  (bind _asbp_player_character (Utilities|Casting|CastToBP_PlayerCharacter (Game|GetPlayerCharacter 0)))
  (return (Variables|/Game/Blueprints/Weapons/BP_WeaponBase.BP_WeaponBase_C|GetWeaponDamage (Variables|/Game/Imports/PlayerCharacter/BP_PlayerCharacter.BP_PlayerCharacter_C|GetCurrentWeapon _asbp_player_character))))