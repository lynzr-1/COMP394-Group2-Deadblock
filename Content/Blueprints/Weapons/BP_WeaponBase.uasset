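; Base weapon actor that the player picks up by interacting, with unarmed, melee, ranged and pistol behavior chosen by WeaponType.
; Equipping drops the current weapon, sets the player's attack montage and snaps armed types' meshes to hand sockets with physics off.
; Dropping detaches the mesh, restores physics and resets animation to unarmed.
; Melee collider overlaps damage zombies, while FireBullet spawns a bullet at AmmoSocket with sound for guns.
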(event OnComponentBeginOverlap(HitCollider)
  (params (OverlappedComponent :type Primitive%20Component%20Object%20Reference) (OtherActor :type Actor%20Object%20Reference) (OtherComp :type Primitive%20Component%20Object%20Reference) (OtherBodyIndex :type Integer) (bFromSweep :type Boolean) (SweepResult :type Hit%20Result%20Structure%20%28by%20ref%29))
  (if (Utilities|Enum|Equal(Enum) (Variables|Default|GetWeaponType) "NewEnumerator1")
    (bind _asbp_zombie_master (Utilities|Casting|CastToBP_ZombieMaster OtherActor))
    (Default|TakeDamage _asbp_zombie_master (Variables|Default|GetWeaponDamage))))

(event EventInteract
  (CallFunction|EquipWeapon))

(fn ConstructionScript)

(fn EquipWeapon
  (bind _weaponmesh (Variables|Default|GetWeaponMesh))
  (bind _weaponmesh_2 (Variables|Default|GetWeaponMesh))
  (bind _asbp_player_character (Utilities|Casting|CastToBP_PlayerCharacter (Game|GetPlayerCharacter 0)))
  (Utilities|IsValid (Variables|/Game/Imports/PlayerCharacter/BP_PlayerCharacter.BP_PlayerCharacter_C|GetCurrentWeapon _asbp_player_character)
    (:Is%20Valid
      (CallFunction|DropWeapon (Variables|/Game/Imports/PlayerCharacter/BP_PlayerCharacter.BP_PlayerCharacter_C|GetCurrentWeapon _asbp_player_character)))
    (:Is%20Not%20Valid
      _))
  (Variables|/Game/Imports/PlayerCharacter/BP_PlayerCharacter.BP_PlayerCharacter_C|SetCurrentWeapon _asbp_player_character self)
  (switch Utilities|FlowControl|Switch|SwitchonE_WeaponType (Variables|Default|GetWeaponType)
    (:NewEnumerator0
      (Variables|/Game/Imports/PlayerCharacter/BP_PlayerCharacter.BP_PlayerCharacter_C|SetCurrentAttackMontage _asbp_player_character "/Game/Imports/PlayerCharacter/Animations/Montage_UnarmedAttack.Montage_UnarmedAttack"))
    (:NewEnumerator1
      (Variables|/Game/Imports/PlayerCharacter/BP_PlayerCharacter.BP_PlayerCharacter_C|SetCurrentAttackMontage _asbp_player_character "/Game/Imports/PlayerCharacter/Animations/Montage_MeleeAttack.Montage_MeleeAttack")
      (Transformation|AttachComponentToComponent _weaponmesh (Variables|/Script/Engine.Character|GetMesh _asbp_player_character) "RightHandSocket" "SnapToTarget" "SnapToTarget" "SnapToTarget" true)
      (Physics|SetSimulatePhysics _weaponmesh_2 false :!label _label)
      (Collision|SetCollisionEnabled _weaponmesh_2 "NoCollision")
      (bind _asbp_player_character_2 (Utilities|Casting|CastToBP_PlayerCharacter (Game|GetPlayerCharacter 0)))
      (Variables|/Game/Imports/PlayerCharacter/BP_PlayerCharacter.BP_PlayerCharacter_C|SetCurrentWeapon _asbp_player_character_2 self)
      (Variables|/Game/Imports/PlayerCharacter/BP_PlayerCharacter.BP_PlayerCharacter_C|SetCurrentInteractable _asbp_player_character_2 0))
    (:NewEnumerator2
      (Variables|/Game/Imports/PlayerCharacter/BP_PlayerCharacter.BP_PlayerCharacter_C|SetCurrentAttackMontage _asbp_player_character "/Game/Imports/PlayerCharacter/Animations/Montage_RangedAttack.Montage_RangedAttack")
      (Transformation|AttachComponentToComponent _weaponmesh (Variables|/Script/Engine.Character|GetMesh _asbp_player_character) "GunSocket" "SnapToTarget" "SnapToTarget" "SnapToTarget" true)
      (goto _label))
    (:NewEnumerator4
      (Variables|/Game/Imports/PlayerCharacter/BP_PlayerCharacter.BP_PlayerCharacter_C|SetCurrentAttackMontage _asbp_player_character "/Game/Imports/PlayerCharacter/Animations/Montage_PistolAttack.Montage_PistolAttack")
      (Transformation|AttachComponentToComponent _weaponmesh (Variables|/Script/Engine.Character|GetMesh _asbp_player_character) "PistolSocket" "SnapToTarget" "SnapToTarget" "SnapToTarget" true)
      (goto _label))))

(fn DropWeapon
  (bind _weaponmesh (Variables|Default|GetWeaponMesh))
  (Transformation|DetachFromComponent _weaponmesh "KeepWorld" "KeepWorld" "KeepWorld" true)
  (Collision|SetCollisionEnabled _weaponmesh "QueryAndPhysics")
  (Physics|SetSimulatePhysics _weaponmesh true)
  (bind _asbp_player_character (Utilities|Casting|CastToBP_PlayerCharacter (Game|GetPlayerCharacter 0)))
  (Variables|/Game/Imports/PlayerCharacter/BP_PlayerCharacter.BP_PlayerCharacter_C|SetCurrentWeapon _asbp_player_character 0)
  (bind _asabp_player_character (Utilities|Casting|CastToABP_PlayerCharacter (Components|SkeletalMesh|GetAnimInstance (Variables|/Script/Engine.Character|GetMesh _asbp_player_character))))
  (Variables|/Game/Imports/PlayerCharacter/Animations/ABP_PlayerCharacter.ABP_PlayerCharacter_C|SetAnimWeaponType _asabp_player_character "NewEnumerator0"))

(fn FireBullet
  (bind _weaponmesh (Variables|Default|GetWeaponMesh))
  (bind _weapontype (Variables|Default|GetWeaponType))
  (if (or (Utilities|Enum|Equal(Enum) _weapontype "NewEnumerator2") (Utilities|Enum|Equal(Enum) _weapontype "NewEnumerator4"))
    (Game|SpawnActorfromClass "/Game/Blueprints/Weapons/BP_Bullet.BP_Bullet_C" (Math|Transform|MakeTransform (Transformation|GetSocketLocation _weaponmesh "AmmoSocket") (Transformation|GetSocketRotation _weaponmesh "AmmoSocket") "1.000000,1.000000,1.000000") "Undefined" "MultiplyWithRoot" 0 0)
    (Audio|PlaySoundatLocation "/Game/Audio/SFX/Weapons/Guns/FireBullet_SoundCue.FireBullet_SoundCue" (Transformation|GetActorLocation) "0, 0, 0" 1.0 1.0 0.0 0 0 0 0)))

(fn GetWeaponDamage
  (return (Variables|Default|GetWeaponDamage)))