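; Base consumable actor that restores the player's health or stamina when interacted with.
; The Interact event switches on ConsumableType, calling Heal or RestoreStamina, which add a clamped amount to BP_PlayerCharacter, refresh the matching HUD bar and destroy the item.
; Healing items also increment a med-kit usage counter on BP_ThirdPersonGameMode before healing.
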(event EventInteract
  (switch Utilities|FlowControl|Switch|SwitchonE_ConsumableType (Variables|Default|GetConsumableType)
    (:NewEnumerator0
      (CallFunction|CountMedKitsUsed)
      (CallFunction|Heal))
    (:NewEnumerator1
      (CallFunction|RestoreStamina))))

(fn ConstructionScript)

(fn Heal
  (bind _asbp_player_character (Utilities|Casting|CastToBP_PlayerCharacter (Game|GetPlayerCharacter 0)))
  (Variables|/Game/Imports/PlayerCharacter/BP_PlayerCharacter.BP_PlayerCharacter_C|SetCurrentHealth _asbp_player_character (Math|Float|Clamp(Float) (+ (Variables|/Game/Imports/PlayerCharacter/BP_PlayerCharacter.BP_PlayerCharacter_C|GetCurrentHealth _asbp_player_character) (Variables|Default|GetHealingAmount)) 0.0 (Variables|/Game/Imports/PlayerCharacter/BP_PlayerCharacter.BP_PlayerCharacter_C|GetMaxHealth _asbp_player_character)))
  (Default|GetHealthPercentage _asbp_player_character)
  (Default|UpdateHealthBar (Variables|/Game/Imports/PlayerCharacter/BP_PlayerCharacter.BP_PlayerCharacter_C|GetHUDWidget _asbp_player_character))
  (Actor|DestroyActor))

(fn RestoreStamina
  (bind _asbp_player_character (Utilities|Casting|CastToBP_PlayerCharacter (Game|GetPlayerCharacter 0)))
  (Variables|/Game/Imports/PlayerCharacter/BP_PlayerCharacter.BP_PlayerCharacter_C|SetCurrentStamina _asbp_player_character (Math|Float|Clamp(Float) (+ (Variables|/Game/Imports/PlayerCharacter/BP_PlayerCharacter.BP_PlayerCharacter_C|GetCurrentStamina _asbp_player_character) (Variables|Default|GetStaminaAmount)) 0.0 (Variables|/Game/Imports/PlayerCharacter/BP_PlayerCharacter.BP_PlayerCharacter_C|GetMaxStamina _asbp_player_character)))
  (Default|GetStaminaPercentage _asbp_player_character)
  (Default|UpdateStaminaBar (Variables|/Game/Imports/PlayerCharacter/BP_PlayerCharacter.BP_PlayerCharacter_C|GetHUDWidget _asbp_player_character))
  (Actor|DestroyActor))

(fn CountMedKitsUsed
  (if (Utilities|Enum|Equal(Enum) (Variables|Default|GetConsumableType) "NewEnumerator0")
    (bind _asbp_third_person_game_mode (Utilities|Casting|CastToBP_ThirdPersonGameMode (Game|GetGameMode)))
    (Variables|/Game/ThirdPerson/Blueprints/BP_ThirdPersonGameMode.BP_ThirdPersonGameMode_C|SetMedKitUsedCount _asbp_third_person_game_mode (+ (Variables|/Game/ThirdPerson/Blueprints/BP_ThirdPersonGameMode.BP_ThirdPersonGameMode_C|GetMedKitUsedCount _asbp_third_person_game_mode) 1))))