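; Zombie spawner actor that periodically spawns random zombie types while its tracked count is below a maximum.
; A looping timer calls SpawnZombie, which places each one at spawn-radius distance in a random 3D direction and passes itself as SpawnerReference.
; RemoveZombieFromArray lets destroyed zombies free their slots.
; After each spawn, the spawner rotates itself from a stored location toward the player, leaving the new zombie's rotation untouched.
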(event EventBeginPlay
  (Utilities|Time|SetTimerbyFunctionName 0 "SpawnZombie" (Variables|Default|GetSpawnInterval) true))

(event Collision|EventActorBeginOverlap
  (params (OtherActor :type Actor%20Object%20Reference)))

(event EventTick
  (params (DeltaSeconds :type Float%20%28single-precision%29)))

(fn ConstructionScript)

(fn SpawnZombie
  (if (< (Utilities|Array|Length (Variables|Default|GetCurrentZombies)) (Variables|Default|GetMaxZombies))
    (bind _returnvalue (Game|SpawnActorfromClass (.OutItem (Utilities|Array|Random (Variables|Default|GetZombieTypes))) (Math|Conversions|ToTransform(Vector) (+ (Transformation|GetActorLocation) (* (Math|Random|RandomUnitVector) (Variables|Default|GetSpawnRadius)))) "Undefined" "MultiplyWithRoot" 0 self 0))
    (Utilities|Array|Add (Variables|Default|GetCurrentZombies) _returnvalue)
    (bind _asbp_player_character (Utilities|Casting|CastToBP_PlayerCharacter (Game|GetPlayerCharacter 0)))
    (Transformation|SetActorRotation (Math|Rotator|FindLookatRotation (Variables|Default|GetSpawnerLocation) (Transformation|GetActorLocation _asbp_player_character)))))

(fn RemoveZombiefromArray
  (params (DestroyedZombie :type BP%20Zombie%20Master%20Object%20Reference))
  (Utilities|Array|RemoveItem (Variables|Default|GetCurrentZombies) DestroyedZombie))