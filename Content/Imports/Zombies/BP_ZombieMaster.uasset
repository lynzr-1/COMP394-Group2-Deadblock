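; Base zombie Character that chases the player through AI MoveTo on spawn, or idles if the game is over.
; Overlap colliders take bullet and weapon damage and start looping attack timers near the player or barricades; only player attacks deal damage.
; Health reaching exactly zero triggers Die, which, given a valid spawner, deregisters and destroys the zombie, increments the GameMode kill count and rolls for loot or weapon drops.
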(event OnComponentBeginOverlap(PlayerDetectCollider)
  (params (OverlappedComponent :type Primitive%20Component%20Object%20Reference) (OtherActor :type Actor%20Object%20Reference) (OtherComp :type Primitive%20Component%20Object%20Reference) (OtherBodyIndex :type Integer) (bFromSweep :type Boolean) (SweepResult :type Hit%20Result%20Structure%20%28by%20ref%29))
  (bind _asbp_player_character (Utilities|Casting|CastToBP_PlayerCharacter OtherActor))
  (if (Class|PrimitiveComponent|IsOverlappingComponent (Variables|Default|GetPlayerDetectCollider) (Variables|/Game/Imports/PlayerCharacter/BP_PlayerCharacter.BP_PlayerCharacter_C|GetZombieAttackDetectRadius _asbp_player_character))
    (Development|PrintString "PLAYER DETECTED...ATTACKING")
    (CallFunction|StartAttacking)))

(event OnComponentBeginOverlap(ZombieHitCollider)
  (params (OverlappedComponent :type Primitive%20Component%20Object%20Reference) (OtherActor :type Actor%20Object%20Reference) (OtherComp :type Primitive%20Component%20Object%20Reference) (OtherBodyIndex :type Integer) (bFromSweep :type Boolean) (SweepResult :type Hit%20Result%20Structure%20%28by%20ref%29))
  (if (Actor|ActorHasTag OtherActor "Bullet")
    (bind _asbp_bullet (Utilities|Casting|CastToBP_Bullet OtherActor))
    (CallFunction|TakeDamage (Variables|/Game/Blueprints/Weapons/BP_Bullet.BP_Bullet_C|GetBulletDamage _asbp_bullet))
    (else
      (bind _asbp_weapon_base (Utilities|Casting|CastToBP_WeaponBase OtherActor))
      (if (and (Utilities|Enum|Equal(Enum) (Variables|/Game/Blueprints/Weapons/BP_WeaponBase.BP_WeaponBase_C|GetWeaponType _asbp_weapon_base) "NewEnumerator1") (Class|PrimitiveComponent|IsCollisionEnabled (Variables|/Game/Blueprints/Weapons/BP_WeaponBase.BP_WeaponBase_C|GetHitCollider _asbp_weapon_base)))
        (CallFunction|TakeDamage (Variables|/Game/Blueprints/Weapons/BP_WeaponBase.BP_WeaponBase_C|GetWeaponDamage _asbp_weapon_base))))))

(event OnComponentEndOverlap(PlayerDetectCollider)
  (params (OverlappedComponent :type Primitive%20Component%20Object%20Reference) (OtherActor :type Actor%20Object%20Reference) (OtherComp :type Primitive%20Component%20Object%20Reference) (OtherBodyIndex :type Integer))
  (bind _asbp_player_character (Utilities|Casting|CastToBP_PlayerCharacter OtherActor))
  (CallFunction|StopAttacking))

(event OnComponentBeginOverlap(ZombieBarrierDetect)
  (params (OverlappedComponent :type Primitive%20Component%20Object%20Reference) (OtherActor :type Actor%20Object%20Reference) (OtherComp :type Primitive%20Component%20Object%20Reference) (OtherBodyIndex :type Integer) (bFromSweep :type Boolean) (SweepResult :type Hit%20Result%20Structure%20%28by%20ref%29))
  (bind _asbp_barricade_base (Utilities|Casting|CastToBP_BarricadeBase OtherActor))
  (if (Class|PrimitiveComponent|IsOverlappingComponent (Variables|/Game/Blueprints/Barricades/BP_BarricadeBase.BP_BarricadeBase_C|GetBarricadeCollider _asbp_barricade_base) (Variables|Default|GetZombieBarrierDetect))
    (CallFunction|StartAttackingBarrier)))

(event OnComponentEndOverlap(ZombieBarrierDetect)
  (params (OverlappedComponent :type Primitive%20Component%20Object%20Reference) (OtherActor :type Actor%20Object%20Reference) (OtherComp :type Primitive%20Component%20Object%20Reference) (OtherBodyIndex :type Integer))
  (bind _asbp_barricade_base (Utilities|Casting|CastToBP_BarricadeBase OtherActor))
  (CallFunction|StopAttackingBarrier))

(event Custom|StartAttacking
  (Utilities|Time|SetTimerbyFunctionName 0 "Attack" 1.5 true))

(event Custom|StopAttacking
  (Utilities|Time|ClearTimerbyFunctionName 0 "Attack"))

(event Custom|StartAttackingBarrier
  (Utilities|Time|SetTimerbyFunctionName 0 "AttackBarrier" 1.5 true))

(event Custom|StopAttackingBarrier
  (Utilities|Time|ClearTimerbyFunctionName 0 "AttackBarrier"))

(event EventBeginPlay
  (bind _asbp_third_person_game_mode (Utilities|Casting|CastToBP_ThirdPersonGameMode (Game|GetGameMode)))
  (if (Variables|/Game/ThirdPerson/Blueprints/BP_ThirdPersonGameMode.BP_ThirdPersonGameMode_C|GetisGameOver _asbp_third_person_game_mode)
    (AI|Navigation|StopMovement (AI|GetAIController self))
    (Animation|PlayAnimMontage "/Game/Imports/Zombies/Animations/Zombie_Idle_Montage.Zombie_Idle_Montage" 1.0 "ZombieIdle")
    (else
      (bind _asbp_player_character (Utilities|Casting|CastToBP_PlayerCharacter (Game|GetPlayerCharacter 0)))
      (AI|AIMoveTo self "0, 0, 0" _asbp_player_character 5e+01 true))))

(fn ConstructionScript
  (Variables|Default|SetZombieCurrentHealth (Variables|Default|GetZombieMaxHealth))
  (Variables|/Script/Engine.CharacterMovementComponent|SetMaxWalkSpeed (Variables|Character|GetCharacterMovement) (Variables|Default|GetZombieSpeed)))

(fn TakeDamage
  (params (IncomingDamage :type Float%20%28double-precision%29))
  (bind _output_get (Variables|Default|SetZombieCurrentHealth (- (Variables|Default|GetZombieCurrentHealth) IncomingDamage)))
  (Animation|PlayAnimMontage "/Game/Imports/Zombies/Animations/ZombieHitReact_Montage.ZombieHitReact_Montage" 1.0 "ZombieHitReact")
  (if (== _output_get 0.0)
    (CallFunction|Die)))

(fn Die
  (bind _spawnerreference (Variables|Default|GetSpawnerReference))
  (Utilities|IsValid _spawnerreference
    (:Is%20Valid
      (Default|RemoveZombiefromArray _spawnerreference self)
      (Actor|DestroyActor)
      (bind _asbp_third_person_game_mode (Utilities|Casting|CastToBP_ThirdPersonGameMode (Game|GetGameMode)))
      (Variables|/Game/ThirdPerson/Blueprints/BP_ThirdPersonGameMode.BP_ThirdPersonGameMode_C|SetZombieKillCount _asbp_third_person_game_mode (+ (Variables|/Game/ThirdPerson/Blueprints/BP_ThirdPersonGameMode.BP_ThirdPersonGameMode_C|GetZombieKillCount _asbp_third_person_game_mode) 1))
      (if (<= (Math|Random|RandomIntegerinRange 1 100) 20)
        (CallFunction|GetRandomLootDrop)
        (elif (<= (Math|Random|RandomIntegerinRange 1 100) 5)
          (CallFunction|GetRandomWeaponDrop))))))

(fn GetRandomLootDrop
  (Game|SpawnActorfromClass (.OutItem (Utilities|Array|Random (Variables|Default|GetLootDrops))) (Math|Conversions|ToTransform(Vector) (Transformation|GetActorLocation)) "Undefined" "MultiplyWithRoot" 0 0))

(fn GetRandomWeaponDrop
  (Game|SpawnActorfromClass (.OutItem (Utilities|Array|Random (Variables|Default|GetWeaponDrops))) (Math|Conversions|ToTransform(Vector) (Transformation|GetActorLocation)) "Undefined" "MultiplyWithRoot" 0 0))

(fn Attack
  (if (not (Variables|Default|GetzIsAttacking))
    (Variables|Default|SetzIsAttacking true)
    (Animation|PlayAnimMontage "/Game/Imports/Zombies/Animations/ZombieAttackMontage.ZombieAttackMontage" 1.0 "zAttack")
    (bind _asbp_player_character (Utilities|Casting|CastToBP_PlayerCharacter (Game|GetPlayerCharacter 0)))
    (Default|TakeDamage _asbp_player_character (Variables|Default|GetZombieDamage))
    (Variables|Default|SetzIsAttacking false)))

(fn MovetoPlayer)

(fn AttackBarrier
  (if (not (Variables|Default|GetzIsAttacking))
    (Variables|Default|SetzIsAttacking true)
    (Animation|PlayAnimMontage "/Game/Imports/Zombies/Animations/ZombieAttackMontage.ZombieAttackMontage" 1.0 "zAttack")
    (Variables|Default|SetzIsAttacking false)))